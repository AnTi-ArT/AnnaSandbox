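; BP_RadialMenu is an actor that shows a radial menu through widget components, with segment count and selection driven by input actions.
; On BeginPlay it gets the dynamic material from WBP_RadialMenu's background image and feeds it Pieces and Selected as scalar parameters.
; RadialMore and RadialLess destroy and respawn item widgets at segment centres using sine and cosine.
; RadialForward advances the selection, resetting it once it exceeds the segment count.
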(event `InputAction|RadialMore`
  (params (Key :type "Key Structure"))
  (bind _items (`self.Items`))
  (bind _radius (`self.Radius`))
  (bind _pieces (`self.Pieces`))
  (bind _returnvalue (/ 360.0 _pieces))
  (:`Released`
    (`/Engine/EditorBlueprintResources/StandardMacros.IncrementFloat` (`self.Pieces`)
      (:`  `
        (`MaterialInstanceDynamic.SetScalarParameterValue` (`self.BG_MAterial`) "Pieces" (`self.Pieces`) :!label _label)
        (for _array_element _items
          (`ActorComponent.K2_DestroyComponent` _array_element))
        (`KismetArrayLibrary.Array_Clear` _items)
        (for _index (range (`KismetMathLibrary.FTrunc` _pieces)) :!label _label_2
          (bind _output_get (set `self.Angle` (+ (* _returnvalue (`KismetMathLibrary.Conv_IntToDouble` _index)) (/ _returnvalue 2.0))))
          (bind _returnvalue_2 (`AddComponent|NODE_AddWidgetComponent-0` :`RelativeTransform` (`KismetMathLibrary.MakeTransform` (`KismetMathLibrary.MakeVector` 5.0 (* (`KismetMathLibrary.DegCos` _output_get) _radius) (* (`KismetMathLibrary.DegSin` _output_get) _radius)) (struct) (0.06 0.06 0.06))))
          (`KismetSystemLibrary.PrintString` (`KismetSystemLibrary.GetDisplayName` _returnvalue_2))
          (`KismetArrayLibrary.Array_Add` (`self.Items`) _returnvalue_2))))))

(event `InputAction|RadialLess`
  (params (Key :type "Key Structure"))
  (:`Released`
    (`/Engine/EditorBlueprintResources/StandardMacros.DecrementFloat` (`self.Pieces`)
      (:`  `
        (goto _label)))))

(event `InputAction|RadialForward`
  (params (Key :type "Key Structure"))
  (bind _selected (`self.Selected`))
  (:`Released`
    (`/Engine/EditorBlueprintResources/StandardMacros.IncrementFloat` _selected
      (:`  `
        (if (> _selected (`self.Pieces`))
          (bind _output_get (set `self.Selected` 0.0)))
        (`MaterialInstanceDynamic.SetScalarParameterValue` (`self.BG_MAterial`) "Selected" _output_get)))))

(event `self.ReceiveBeginPlay`
  (`self.EnableInput` (`GameplayStatics.GetPlayerController` 0))
  (bind _aswbp_radial_menu (cast `/Game/A_Testzeug/WBP_RadialMenu` (`WidgetComponent.GetUserWidgetObject` (`self.W_Image`))))
  (bind _returnvalue (`Image.GetDynamicMaterial` (`/Game/A_Testzeug/WBP_RadialMenu.BG_IMG` _aswbp_radial_menu)))
  (bind _output_get (set `self.BG_MAterial` _returnvalue))
  (`MaterialInstanceDynamic.SetScalarParameterValue` _output_get "Selected" (`self.Selected`))
  (`MaterialInstanceDynamic.SetScalarParameterValue` _output_get "Pieces" (`self.Pieces`))
  (goto _label_2))

(fn `UserConstructionScript`)